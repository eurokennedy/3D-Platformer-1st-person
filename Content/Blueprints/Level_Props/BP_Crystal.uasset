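; BP_Crystal is a collectible level prop that can optionally slide back and forth along the world X axis.
; When CanMove is set, Tick moves it by Speed and reverses direction at MaxX and its negative, so the range centers on world zero rather than its placement.
; On overlap with a BP_GameCharacter, it increments that character's CrystalCount and destroys itself.
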(event `self.ReceiveTick`
  (params (DeltaSeconds :type "Float (single-precision)"))
  (bind _returnvalue_x (`KismetMathLibrary.BreakVector` (`self.K2_GetActorLocation`)))
  (bind (_returnvalue_x_2 _returnvalue_y _returnvalue_z) (`KismetMathLibrary.BreakVector` (`self.K2_GetActorLocation`)))
  (bind _returnvalue_x_3 (`KismetMathLibrary.BreakVector` (`self.K2_GetActorLocation`)))
  (if (`self.Can Move`)
    (`self.K2_SetActorLocation` (`KismetMathLibrary.MakeVector` (+ (* (`self.Speed`) DeltaSeconds) _returnvalue_x_2) _returnvalue_y _returnvalue_z))
    (if (>= _returnvalue_x_3 (`self.Max X`))
      (set `self.Speed` (* (`self.Speed`) -1.0))
      (elif (< _returnvalue_x (* (`self.Max X`) -1.0))
        (set `self.Speed` (`KismetMathLibrary.Abs` (`self.Speed`)))))))

(event `self.ReceiveActorBeginOverlap`
  (params (OtherActor :type "Actor Object Reference"))
  (bind _asbp_game_character (cast `/Game/Blueprints/Character_Blueprints/BP_GameCharacter` OtherActor))
  (`/Engine/EditorBlueprintResources/StandardMacros.IncrementInt` (`/Game/Blueprints/Character_Blueprints/BP_GameCharacter.Crystal Count` _asbp_game_character)
    (:`  `
      (`self.K2_DestroyActor`))))

(fn `UserConstructionScript`)