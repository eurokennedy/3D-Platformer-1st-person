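; Door actor that ends the game when the player opens it after collecting three crystals and putting the chair in place.
; Trigger overlap checks both conditions on BP_GameCharacter, sets its on-screen hint and enables the door's input only when both are met.
; Leaving the trigger clears the hint and disables input.
; The Open Door action swings the actor's yaw through a timeline, then calls GameOver on the character.
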(event `self.Door Trigger.OnComponentBeginOverlap`
  (params (OverlappedComponent :type "PrimitiveComponent Object Reference") (OtherActor :type "Actor Object Reference") (OtherComp :type "PrimitiveComponent Object Reference") (OtherBodyIndex :type Integer) (bFromSweep :type Boolean) (SweepResult :type "HitResult Structure (by ref)"))
  (bind _asbp_game_character (cast `/Game/Blueprints/Character_Blueprints/BP_GameCharacter` OtherActor))
  (if (== (`/Game/Blueprints/Character_Blueprints/BP_GameCharacter.Crystal Count` _asbp_game_character) 3)
    (if (`/Game/Blueprints/Character_Blueprints/BP_GameCharacter.ChairInPlace` _asbp_game_character)
      (set `/Game/Blueprints/Character_Blueprints/BP_GameCharacter.CrystalScreenMessage` "Press 'e' to open the door" _asbp_game_character)
      (`self.EnableInput` (`GameplayStatics.GetPlayerController` 0))
      (else
        (set `/Game/Blueprints/Character_Blueprints/BP_GameCharacter.CrystalScreenMessage` "You collected the Crystals, but first you must sit at the table" _asbp_game_character)))
    (else
      (set `/Game/Blueprints/Character_Blueprints/BP_GameCharacter.CrystalScreenMessage` "You need to collect all 3 Crystals to Open the door" _asbp_game_character))))

(event `self.Door Trigger.OnComponentEndOverlap`
  (params (OverlappedComponent :type "PrimitiveComponent Object Reference") (OtherActor :type "Actor Object Reference") (OtherComp :type "PrimitiveComponent Object Reference") (OtherBodyIndex :type Integer))
  (bind _asbp_game_character (cast `/Game/Blueprints/Character_Blueprints/BP_GameCharacter` OtherActor))
  (set `/Game/Blueprints/Character_Blueprints/BP_GameCharacter.CrystalScreenMessage` "" _asbp_game_character)
  (`self.DisableInput` (`GameplayStatics.GetPlayerController` 0)))

(event `InputAction|Open Door`
  (params (Key :type "Key Structure"))
  (:`Pressed`
    (set `self.Initial Rotation` (`self.K2_GetActorRotation`))
    (bind (_direction _rotate_z) (`Timeline|Z Rotation Timeline`)
      (:`Update`
        (`self.K2_SetActorRotation` (`KismetMathLibrary.MakeRotator` (.roll (`self.Initial Rotation`)) (.pitch (`self.Initial Rotation`)) (- (.yaw (`self.Initial Rotation`)) _rotate_z))))
      (:`Finished`
        (`/Game/Blueprints/Character_Blueprints/BP_GameCharacter.Game Over` (stale `self.Door Trigger.OnComponentBeginOverlap` _asbp_game_character))))))

(fn `UserConstructionScript`)